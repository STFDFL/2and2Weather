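; Mouse-driven player controller for placing a wind by press-and-drag between two cursor-traced points.
; Press spawns the origin marker; release spawns the direction marker and a particle effect, rotating origin and effect toward it.
; Tick then fires once, spawning WindForce at a fixed world-X offset from the origin, with debug drawing.
; Cancel destroys markers and effect but not WindForce; speed inputs only change and print WindSpeed.
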(event EventTick
  (params (DeltaSeconds :type Float%20%28single-precision%29))
  (if (Variables|Default|GetWindParametersSet)
    (Class|KismetSystemLibrary|LineTraceMultiNEW (stale Input|ActionEvents|InputActionSetWindButton _output_get) (stale Input|ActionEvents|InputActionSetWindButton _output_get_2) "TraceTypeQuery2" false 0 "ForDuration" true)
    (Variables|Default|SetWindIsSpawned true)
    (CallFunction|SpawnWindForce)
    (Variables|Default|SetWindParametersSet false)))

(event Input|ActionEvents|InputActionSetWindButton
  (params (Key :type Key%20Structure :default "AnyKey"))
  ;[1 1 1] IF the spawning point of the wind is...
  (:Pressed
    (Variables|Default|SetisCharging true)
    (if (not (Variables|Default|GetWindIsSpawned))
      ;[1 1 1] ...NOT set, with this code set the wind spawning point, spawn a cylinder
      (bind _output_get (Variables|Default|SetWindSpawnLocation (.Location (Collision|BreakHitResult (.HitResult (Game|Player|GetHitResultUnderCursorbyChannel "TraceTypeQuery1" true))))))
      (Variables|Default|SetWindASpotIsSet true)
      (bind _returnvalue (Game|SpawnActorfromClass "/Game/Blueprints/WindSpawnPoint.WindSpawnPoint_C" (Math|Conversions|ToTransform(Vector) _output_get) "AlwaysSpawn" 0 0))
      (Variables|Default|SetWindSpawnPoint _returnvalue)))
  (:Released
    (Variables|Default|SetisCharging false)
    (if (not (Variables|Default|GetWindIsSpawned))
      ;[1 1 1] IS set, with this code set the wind direction point, spawn another cylinder
      (bind _output_get_2 (Variables|Default|SetWindDirection (.Location (Collision|BreakHitResult (.HitResult (Game|Player|GetHitResultUnderCursorbyChannel "TraceTypeQuery1" true))))))
      (Variables|Default|SetWindBSpotIsSet true)
      (bind _returnvalue_2 (Game|SpawnActorfromClass "/Game/Blueprints/WindDirectionPoint.WindDirectionPoint_C" (Math|Conversions|ToTransform(Vector) _output_get_2) "AlwaysSpawn" 0 0))
      (Variables|Default|SetWindDirectionPoint _returnvalue_2)
      (Variables|Default|SetWindParametersSet true)
      (Transformation|SetActorRotation (Variables|Default|GetWindSpawnPoint) (Math|Rotator|FindLookatRotation (Transformation|GetActorLocation (Variables|Default|GetWindSpawnPoint)) (Transformation|GetActorLocation (Variables|Default|GetWindDirectionPoint))))
      (bind _returnvalue_3 (Game|SpawnActorfromClass "/Game/Blueprints/WindParticleEffect.WindParticleEffect_C" (Math|Conversions|ToTransform(Vector) (Transformation|GetActorLocation (Variables|Default|GetWindSpawnPoint))) "Undefined" 0 0))
      (Transformation|SetActorRotation _returnvalue_3 (Math|Rotator|FindLookatRotation (Transformation|GetActorLocation (Variables|Default|GetWindSpawnPoint)) (Transformation|GetActorLocation (Variables|Default|GetWindDirectionPoint))))
      (Variables|Default|SetWindEffect _returnvalue_3))))

(event Input|ActionEvents|InputActionCancelWind
  (params (Key :type Key%20Structure :default "AnyKey"))
  ;[1 1 1] Cancel Wind
  (:Pressed
    (if (Variables|Default|GetWindIsSpawned)
      (Variables|Default|SetWindASpotIsSet false)
      (Variables|Default|SetWindBSpotIsSet false)
      (Variables|Default|SetWindParametersSet false)
      (Variables|Default|SetWindIsSpawned false)
      (Actor|DestroyActor (Variables|Default|GetWindSpawnPoint))
      (Actor|DestroyActor (Variables|Default|GetWindDirectionPoint))
      (Actor|DestroyActor (Variables|Default|GetWindEffect)))))

(event Input|ActionEvents|InputActionIncreaseWindSpeed
  (params (Key :type Key%20Structure :default "AnyKey"))
  ;[1 1 1] Increase / Decrease wind speed
  (:Pressed
    (bind _output_get (Variables|Default|SetWindSpeed (+ (Variables|Default|GetWindSpeed) 5e+01)))
    (Development|PrintString (Utilities|String|ToString(Float) _output_get))))

(event Input|ActionEvents|InputActionDecreaseWindSpeed
  (params (Key :type Key%20Structure :default "AnyKey"))
  ;[1 1 1] Increase / Decrease wind speed
  (:Pressed
    (bind _output_get (Variables|Default|SetWindSpeed (- (Variables|Default|GetWindSpeed) 5e+01)))
    (Development|PrintString (Utilities|String|ToString(Float) _output_get))))

(fn ConstructionScript)

(fn SpawnWindForce
  (bind _windspawnpoint (Variables|Default|GetWindSpawnPoint))
  (bind _returnvalue (Transformation|GetActorLocation _windspawnpoint))
  (bind _returnvalue_2 (- _returnvalue "500.000000, 0, 0"))
  (Game|SpawnActorfromClass "/Game/Blueprints/WindForce.WindForce_C" (Math|Conversions|ToTransform(Vector) _returnvalue_2) "AlwaysSpawn" 0 0)
  (Rendering|Debug|DrawDebugSphere _returnvalue_2 1e+02 12 "(R=1.000000,G=1.000000,B=1.000000,A=1.000000)" 2e+01))