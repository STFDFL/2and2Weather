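; Floor actor that simulates getting wet and drying through material parameters on its static mesh.
; The construction script creates a dynamic material instance; while IsGettingWet is set, Tick uses a Delay to lower roughness in steps and raise a metal counter.
; DryFloor clears the flag, so Tick snaps both values back to dry defaults.
; The FloorMetal parameter is always written as 1.0, regardless of the counter.
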(event EventBeginPlay
  ;[1 1 1] Enable Inputs
  (Input|EnableInput (Game|GetPlayerController 0))
  ;[1 1 1] Make the floor wet
  ;;[1 1 1] Decrease roughness over time
  (bind _output_get (Variables|Default|SetFloorRoughnessValue (- (Variables|Default|GetFloorRoughnessValue) 0.05)))
  (Rendering|Material|SetScalarParameterValueonMaterials (Variables|Debug|GetStaticMeshComponent) "Metalness Roughness" _output_get)
  ;;[1 1 1] add metalness
  (if (< (Variables|Default|GetFloorMetalValue) 0.8)
    (Variables|Default|SetFloorMetalValue (+ (Variables|Default|GetFloorMetalValue) 0.05))
    (Rendering|Material|SetScalarParameterValueonMaterials (Variables|Debug|GetStaticMeshComponent) "FloorMetal" 1.0)))

(event Collision|EventActorBeginOverlap
  (params (OtherActor :type Actor%20Object%20Reference)))

(event EventTick
  (params (DeltaSeconds :type Float%20%28single-precision%29))
  (if (Variables|Default|GetIsGettingWet)
    ;[1 1 1] Make the floor wet
    ;;[1 1 1] Decrease roughness over time
    (Utilities|FlowControl|Delay 0.4)
    (if (> (Variables|Default|GetFloorRoughnessValue) 0.0)
      (bind _output_get (Variables|Default|SetFloorRoughnessValue (- (Variables|Default|GetFloorRoughnessValue) 0.05)))
      (Rendering|Material|SetScalarParameterValueonMaterials (Variables|Debug|GetStaticMeshComponent) "Metalness Roughness" _output_get)
      ;;[1 1 1] add metalness
      (if (< (Variables|Default|GetFloorMetalValue) 0.8)
        (Variables|Default|SetFloorMetalValue (+ (Variables|Default|GetFloorMetalValue) 0.05))
        (Rendering|Material|SetScalarParameterValueonMaterials (Variables|Debug|GetStaticMeshComponent) "FloorMetal" 1.0)))
    (else
      ;[1 1 1] Decrease roughness over time
      (bind _output_get_2 (Variables|Default|SetFloorRoughnessValue 1.0))
      (Rendering|Material|SetScalarParameterValueonMaterials (Variables|Debug|GetStaticMeshComponent) "Metalness Roughness" _output_get_2)
      ;[1 1 1] add metalness
      (Variables|Default|SetFloorMetalValue 0.0)
      (Rendering|Material|SetScalarParameterValueonMaterials (Variables|Debug|GetStaticMeshComponent) "FloorMetal" 1.0))))

(fn ConstructionScript
  (bind _returnvalue (Rendering|Material|CreateDynamicMaterialInstance (Variables|Debug|GetStaticMeshComponent) 0 "/Game/GTFreeMaterials/Materials/MasterMaterialStef.MasterMaterialStef" :!class /Script/Engine.PrimitiveComponent))
  (Variables|Default|SetDynamicMaterialFloor _returnvalue)
  (Variables|Default|SetFloorMetalValue 0.0)
  (Variables|Default|SetFloorRoughnessValue 1.0))

(fn DryFloor
  (Variables|Default|SetIsGettingWet false))