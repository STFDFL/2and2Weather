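; RainController is an actor that toggles rain on and off through the ActivateRain input action.
; When wind is active, rain spawns at the wind location from Mouse_PlayerController, oriented toward the wind direction.
; Otherwise it spawns at the FPCharacter's location and flags the floor as getting wet, which the wind branch skips.
; Switching off destroys the rain effect, then dries the floor after a short delay.
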(event EventBeginPlay
  ;[1 1 1] Enable Inputs
  (Input|EnableInput (Game|GetPlayerController 0)))

(event Collision|EventActorBeginOverlap
  (params (OtherActor :type Actor%20Object%20Reference)))

(event Input|ActionEvents|InputActionActivateRain
  (params (Key :type Key%20Structure :default "AnyKey"))
  ;[1 1 1] Check if the rain is already on
  (:Pressed
    (if (Variables|Default|GetRainIsOn)
      ;[1 1 1] Turn Off Rain and dry floor
      (Variables|Default|SetRainIsOn false)
      (Actor|DestroyActor (Variables|Default|GetRainSpawned))
      (Utilities|FlowControl|Delay 3.0)
      (Default|DryFloor (Variables|Default|GetFloorRef))
      (else
        (Variables|Default|SetRainIsOn true)
        (bind _asmouse_player_controller (Utilities|Casting|CastToMouse_PlayerController (Game|GetPlayerController 0)))
        (if (Variables|/Game/Blueprints/Mouse_PlayerController.Mouse_PlayerController_C|GetWindIsSpawned _asmouse_player_controller) ; Check if Wind is On
          ;[1 1 1] Activate Rain when wind is On
          (bind _output_get (Variables|Default|SetRainSpawnLocation (Variables|/Game/Blueprints/Mouse_PlayerController.Mouse_PlayerController_C|GetWindSpawnLocation _asmouse_player_controller)))
          (bind _output_get_2 (Variables|Default|SetRainDirection (Variables|/Game/Blueprints/Mouse_PlayerController.Mouse_PlayerController_C|GetWindDirection _asmouse_player_controller)))
          (bind _returnvalue (Game|SpawnActorfromClass "/Game/Blueprints/RainParticleEffect.RainParticleEffect_C" (Math|Transform|MakeTransform _output_get (Math|Rotator|FindLookatRotation _output_get _output_get_2)) "Undefined" 0 0))
          (Variables|Default|SetRainSpawned _returnvalue)
          (else
            ;[1 1 1] Activate Rain when wind is Off
            (bind _returnvalue_2 (Game|SpawnActorfromClass "/Game/Blueprints/RainParticleEffect.RainParticleEffect_C" (Math|Conversions|ToTransform(Vector) (Transformation|GetActorLocation (Variables|Default|GetFPCharacter))) "Undefined" 0 0))
            (CallFunction|SetGroundWetness)
            (Variables|Default|SetRainSpawned _returnvalue_2)))))))

(fn ConstructionScript)

(fn SetGroundWetness
  (if (Variables|Default|GetRainIsOn)
    (bind _asfloor_blueprint (Utilities|Casting|CastToFloor_Blueprint (Variables|Default|GetFloorRef)))
    (Variables|/Game/Blueprints/Floor_Blueprint.Floor_Blueprint_C|SetIsGettingWet _asfloor_blueprint true)))