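; Physics pick-up actor that lets the player grab, carry and throw objects with the right mouse button.
; A camera line trace, with range adjusted by mouse wheel, attaches a runtime-added PhysicsHandle to objects under a mass limit.
; Tick moves the handle along control rotation from this actor's location, using its world-origin distance as offset.
; Releasing drops the object, with a forward impulse if Q is held; WorldStatic collision stays ignored.
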(event EventBeginPlay
  ;[1 1 1] Enable Inputs
  (Input|EnableInput (Game|GetPlayerController 0)))

(event EventTick
  (params (DeltaSeconds :type Float%20%28single-precision%29))
  (if (Variables|Default|GetPhysics%20Handle%20Active)
    (Variables|Default|SetHandle%20Location (+ (+ (Transformation|GetActorLocation) (* (Math|Vector|GetForwardVector (Pawn|GetControlRotation (Game|GetPlayerController 0) :!class /Script/Engine.Controller)) (Variables|Default|GetOther%20Item%20Location))) "0, 0,50.000000"))
    (Class|PhysicsHandleComponent|SetTargetLocationandRotation (Variables|Default|GetPhysics%20Handle) (Variables|Default|GetHandle%20Location) (Pawn|GetControlRotation (Game|GetPlayerController 0) :!class /Script/Engine.Controller))))

(event Input|MouseEvents|RightMouseButton
  (params (Key :type Key%20Structure :default "AnyKey"))
  (bind _fpcharacterref (Variables|Default|GetFPCharacterRef))
  (bind _firstpersoncamera (Variables|/Game/FirstPersonBP/Blueprints/FirstPersonCharacter.FirstPersonCharacter_C|GetFirstPersonCamera _fpcharacterref))
  (bind _returnvalue (Transformation|GetWorldLocation _firstpersoncamera))
  (:Pressed
    (Variables|Default|SetPhysics%20Handle%20Active true)
    (bind (_outhit _returnvalue_2) (Collision|LineTraceForObjects _returnvalue (+ _returnvalue (* (Math|Vector|GetForwardVector _firstpersoncamera) (Variables|Default|GetPick%20Up%20Distance))) (Utilities|Array|MakeArray (Variables|Default|GetPhysics%20Object%20Types)) false 0 "None"))
    (Variables|Default|SetOther%20Item%20Location (Math|Vector|VectorLength (- (Transformation|GetActorLocation) "0, 0, 0")))
    (Variables|Default|SetOther%20Item%20Rotation (Transformation|GetActorRotation))
    (if _returnvalue_2
      (if (< (Physics|GetMass (.HitComponent (Collision|BreakHitResult _outhit))) 5e+02)
        (bind _returnvalue_3 (AddComponent|AddPhysicsHandleComponent))
        (Variables|Default|SetPhysics%20Handle _returnvalue_3)
        (Variables|Default|SetPhysics%20Object (.HitComponent (Collision|BreakHitResult _outhit)))
        (Class|PhysicsHandleComponent|GrabComponent (Variables|Default|GetPhysics%20Handle) (.HitComponent (Collision|BreakHitResult _outhit)) "None" "0, 0, 0" false)
        (Collision|SetCollisionResponsetoChannel (.HitComponent (Collision|BreakHitResult _outhit)) "ECC_WorldStatic" "ECR_Ignore"))))
  (:Released
    (Variables|Default|SetPhysics%20Handle%20Active false)
    (Physics|Components|PhysicsHandle|ReleaseComponent (Variables|Default|GetPhysics%20Handle))
    (if (Variables|Default|GetIs%20Held?)
      (Physics|AddImpulse (.HitComponent (Collision|BreakHitResult _outhit)) (* (Math|Vector|GetForwardVector (Variables|/Game/FirstPersonBP/Blueprints/FirstPersonCharacter.FirstPersonCharacter_C|GetFirstPersonCamera (Variables|Default|GetFPCharacterRef))) 5e+03) "None" false))
    (Collision|SetCollisionResponsetoChannel (.HitComponent (Collision|BreakHitResult _outhit)) "ECC_WorldStatic" "ECR_Ignore")))

(event Input|KeyboardEvents|Q
  (params (Key :type Key%20Structure :default "AnyKey"))
  (:Pressed
    (Variables|Default|SetIs%20Held? true))
  (:Released
    (Variables|Default|SetIs%20Held? false)))

(event Input|MouseEvents|MouseWheelUp
  (params (Key :type Key%20Structure :default "AnyKey"))
  (:Pressed
    (Variables|Default|SetPick%20Up%20Distance (+ (Variables|Default|GetPick%20Up%20Distance) 25.0))))

(event Input|MouseEvents|MouseWheelDown
  (params (Key :type Key%20Structure :default "AnyKey"))
  (:Pressed
    (Variables|Default|SetPick%20Up%20Distance (- (Variables|Default|GetPick%20Up%20Distance) 25.0))))

(fn ConstructionScript)