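; Hookable cargo actor that a crane arm picks up and drops.
; Overlapping near the crane's hook sphere sets IAmHooked on the CraneArmTop after a short delay, and the DropCargo input clears it.
; Tick reads that flag through the overlapped actor: when hooked, physics and collision go off and the actor follows the hook's offset position and rotation.
; When unhooked, it still sets a position below the hook while re-enabling physics and collision.
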(event Collision|EventActorBeginOverlap
  (params (OtherActor :type Actor%20Object%20Reference))
  (if (< (Math|Vector|VectorLength (- (Transformation|GetWorldLocation (Variables|Default|GetCube)) (Transformation|GetWorldLocation (Variables|/Game/Blueprints/CraneBP/CraneArmTop.CraneArmTop_C|Gettopspherehook (Variables|Default|GetCraneArmTopRef))))) 165.0)
    ;[1 1 1] set the hookable object to hooked
    (bind _ascrane_arm_top (Utilities|Casting|CastToCraneArmTop OtherActor))
    (if (not (Variables|/Game/Blueprints/CraneBP/CraneArmTop.CraneArmTop_C|GetIAmHooked _ascrane_arm_top))
      (Utilities|FlowControl|Delay 0.1)
      (Variables|/Game/Blueprints/CraneBP/CraneArmTop.CraneArmTop_C|SetIAmHooked _ascrane_arm_top true))))

(event EventBeginPlay
  ;[1 1 1] Enable Inputs
  (Input|EnableInput (Game|GetPlayerController 0)))

(event EventTick
  (params (DeltaSeconds :type Float%20%28single-precision%29))
  (bind _cube (Variables|Default|GetCube))
  (bind _cube_2 (Variables|Default|GetCube))
  ;[1 1 1] set the location and physics of the hookable depending of its status (hooked / not hooked)
  (bind _ascrane_arm_top (Utilities|Casting|CastToCraneArmTop (stale Collision|EventActorBeginOverlap OtherActor)))
  (if (Variables|/Game/Blueprints/CraneBP/CraneArmTop.CraneArmTop_C|GetIAmHooked _ascrane_arm_top)
    (Physics|SetSimulatePhysics _cube_2 false)
    (Collision|SetCollisionEnabled _cube_2 "NoCollision")
    (Transformation|SetActorLocation (+ (Transformation|GetWorldLocation (Variables|/Game/Blueprints/CraneBP/CraneArmTop.CraneArmTop_C|Gettopspherehook _ascrane_arm_top)) "0.000000,0.000000,-150.000000") false false)
    ;[1 1 1] set rotation of the hookable when its hooked
    (Transformation|SetActorRotation (Math|Rotator|MakeRotator (.Roll (Math|Rotator|BreakRotator (Transformation|GetWorldRotation (Variables|/Game/Blueprints/CraneBP/CraneArmTop.CraneArmTop_C|Gettopspherehook _ascrane_arm_top)))) (+ (.Pitch (Math|Rotator|BreakRotator (Transformation|GetWorldRotation (Variables|/Game/Blueprints/CraneBP/CraneArmTop.CraneArmTop_C|Gettopspherehook _ascrane_arm_top)))) -35.0) (.Yaw (Math|Rotator|BreakRotator (Transformation|GetWorldRotation (Variables|/Game/Blueprints/CraneBP/CraneArmTop.CraneArmTop_C|Gettopspherehook _ascrane_arm_top))))))
    (else
      (Transformation|SetActorLocation (+ (Transformation|GetWorldLocation (Variables|/Game/Blueprints/CraneBP/CraneArmTop.CraneArmTop_C|Gettopspherehook _ascrane_arm_top)) "0.000000,0.000000,-170.000000") false false)
      (Collision|SetCollisionEnabled _cube "QueryAndPhysics")
      (Physics|SetSimulatePhysics _cube true))))

(event Input|ActionEvents|InputActionDropCargo
  (params (Key :type Key%20Structure :default "AnyKey"))
  (:Pressed
    (Variables|/Game/Blueprints/CraneBP/CraneArmTop.CraneArmTop_C|SetIAmHooked (Variables|Default|GetCraneArmTopRef) false)))

(fn ConstructionScript)