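; CraneArmTop is a crane actor that the player raises and lowers with the extend and retract hook inputs.
; It enables input for player 0, and press and release events set flags that Tick reads, with extend taking priority.
; Each frame moves the whole actor one unit vertically, independent of delta time.
; Both directions require Z above 1000, so retract stops working at that floor.
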(event Collision|EventActorBeginOverlap
  (params (OtherActor :type Actor%20Object%20Reference)))

(event EventBeginPlay
  ;[1 1 1] Enable Inputs
  (Input|EnableInput (Game|GetPlayerController 0)))

(event EventTick
  (params (DeltaSeconds :type Float%20%28single-precision%29))
  (bind _returnvalue (Transformation|GetActorLocation))
  (bind _z (Math|Vector|BreakVector _returnvalue))
  (bind _returnvalue_2 (> _z 1e+03))
  (if (Variables|Default|GetECHIsPressed) ; Extending the hook?
    (if _returnvalue_2
      (Transformation|SetActorLocation (+ (Transformation|GetActorLocation) "0.000000, 0,-1.000000") false false))
    (elif (Variables|Default|GetRCHIsPressed) ; Retracting the hook?
      (if _returnvalue_2
        (Transformation|SetActorLocation (+ (Transformation|GetActorLocation) "0.000000, 0,1.000000") false false)))))

(event Input|ActionEvents|InputActionExtendCraneHook
  (params (Key :type Key%20Structure :default "AnyKey"))
  (:Pressed
    (Variables|Default|SetECHIsPressed true))
  (:Released
    (Variables|Default|SetECHIsPressed false)))

(event Input|ActionEvents|InputActionRetractCraneHook
  (params (Key :type Key%20Structure :default "AnyKey"))
  (:Pressed
    (Variables|Default|SetRCHIsPressed true))
  (:Released
    (Variables|Default|SetRCHIsPressed false)))

(fn ConstructionScript)