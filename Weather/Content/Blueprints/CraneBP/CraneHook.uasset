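; Crane hook actor Blueprint that takes player input for extending and retracting the hook, with the movement itself not yet implemented.
; It enables input from the first player controller on BeginPlay, and the two input actions set held-state flags on press and release.
; Tick prints the distance to the Cable as debug output and checks the flags in nested branches that do nothing.
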(event Collision|EventActorBeginOverlap
  (params (OtherActor :type Actor%20Object%20Reference)))

(event EventTick
  (params (DeltaSeconds :type Float%20%28single-precision%29))
  (Development|PrintString (Utilities|String|ToString(Float) (Transformation|GetDistanceTo (Variables|Default|GetCable))))
  (if (Variables|Default|GetisPageUpPressed)
    (if (Variables|Default|GetisPageDownPressed)
      _)))

(event EventBeginPlay
  ;[1 1 1] Enable Inputs
  (Input|EnableInput (Game|GetPlayerController 0)))

(event Input|ActionEvents|InputActionExtendCraneHook
  (params (Key :type Key%20Structure :default "AnyKey"))
  (:Pressed
    (Variables|Default|SetisPageUpPressed true))
  (:Released
    (Variables|Default|SetisPageUpPressed false)))

(event Input|ActionEvents|InputActionRetractCraneHook
  (params (Key :type Key%20Structure :default "AnyKey"))
  (:Pressed
    (Variables|Default|SetisPageDownPressed true))
  (:Released
    (Variables|Default|SetisPageDownPressed false)))

(fn ConstructionScript)